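; Animation notify that plays a Wwise footstep sound and a camera shake when triggered.
; It sets the surface switch to a fixed concrete value and posts the footstep event on the owning actor.
; Horizontal velocity then selects a walk or run world camera shake centred on the actor, with a debug print naming the chosen gait.
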(fn OnReceiveNotify
  (params (OwningInstance :type Paper%20ZD%20Anim%20Instance%20Object%20Reference))
  (bind _returnvalue (Class|PaperZDAnimInstance|GetOwningActor OwningInstance))
  (bind _returnvalue_2 (Transformation|GetVelocity _returnvalue))
  (bind _returnvalue_3 (Transformation|GetActorLocation _returnvalue))
  (bind (_x _y) (Math|Vector|BreakVector _returnvalue_2))
  (Class|AkGameplayStatics|SetSwitch "/Game/WwiseAudio/Switches/Default_Work_Unit/Material/Material-Concrete.Material-Concrete" _returnvalue)
  (Class|AkGameplayStatics|PostEvent "/Game/WwiseAudio/Events/Player_Audio_Events/Movement/Play_Footsteps.Play_Footsteps" _returnvalue)
  (if (<= (Math|Vector|VectorLength (Math|Vector|MakeVector _x _y 0.0)) 6e+02)
    (Camera|PlayWorldCameraShake (Variables|Default|GetWalk%20Camera%20Shake) _returnvalue_3 0.0 1e+03)
    (Development|PrintString "Walk")
    (else
      (Camera|PlayWorldCameraShake (Variables|Default|GetRun%20Camera%20Shake) _returnvalue_3 0.0 1e+03)
      (Development|PrintString "Run"))))